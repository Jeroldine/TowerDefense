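; Actor component that makes a grid tile respond to mouse clicks and cursor hover.
; On BeginPlay it binds to its owner's click and cursor-over events.
; Each event logs a debug string, then forwards to the owner through BPI_InteractableObject messages, leaving build and colour-change behaviour to the owner.
; The MouseClicked and hover functions on the component itself are empty stubs.
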(event `self.ReceiveBeginPlay`
  (bind _returnvalue (`self.GetOwner`))
  (add `Actor.OnClicked` _returnvalue (delegate `Clicked`))
  (add `Actor.OnBeginCursorOver` _returnvalue (delegate `HoverStart`))
  (add `Actor.OnEndCursorOver` _returnvalue (delegate `HoverEnd`)))

(event `Clicked`
  (params (TouchedActor :type "Actor Object Reference") (ButtonPressed :type "Key Structure" :default "None"))
  (`self.Build`))

(event `HoverStart`
  (params (TouchedActor :type "Actor Object Reference"))
  (`self.ChangeColour`))

(event `HoverEnd`
  (params (TouchedActor :type "Actor Object Reference"))
  (`self.RevertColour`))

(fn `Build`
  (bind _returnvalue (`self.GetOwner`))
  (`KismetSystemLibrary.PrintString` "Check to see if you can build")
  (cast `/Game/Blueprints/Helpers/BPI_InteractableObject` _returnvalue)
  (message `/Game/Blueprints/Helpers/BPI_InteractableObject.MouseClicked` _returnvalue))

(fn `ChangeColour`
  (bind _returnvalue (`self.GetOwner`))
  (`KismetSystemLibrary.PrintString` "Changing to appropriate colour")
  (cast `/Game/Blueprints/Helpers/BPI_InteractableObject` _returnvalue)
  (message `/Game/Blueprints/Helpers/BPI_InteractableObject.MouseHoverStart` _returnvalue))

(fn `MouseClicked`)

(fn `MouseHoverEnd`)

(fn `MouseHoverStart`)

(fn `RevertColour`
  (bind _returnvalue (`self.GetOwner`))
  (`KismetSystemLibrary.PrintString` "Reverting color")
  (cast `/Game/Blueprints/Helpers/BPI_InteractableObject` _returnvalue)
  (message `/Game/Blueprints/Helpers/BPI_InteractableObject.MouseHoverEnd` _returnvalue))