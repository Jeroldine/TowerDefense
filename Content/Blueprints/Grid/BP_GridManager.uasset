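; BP_GridManager spawns a grid of BP_Tile actors when play begins and prints debug messages.
; ConstructGrid loops over rows and columns, using a macro to derive each tile's position from its indices and tile size.
; SpawnTile initializes each tile with its indices, dimension and shrink factor, then stores it in TileArray.
; UpdateGrid is an empty stub.
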(event `self.ReceiveBeginPlay`
  (`KismetSystemLibrary.PrintString` "Grid Manager in Scene")
  (`self.ConstructGrid`)
  (`KismetSystemLibrary.PrintString` "Number of elements in grid array" true true (struct :`G` 0.66 :`B` 1.0 :`A` 1.0) 5.0)
  (`KismetSystemLibrary.PrintString` (`KismetStringLibrary.Conv_IntToString` (`KismetArrayLibrary.Array_Length` (`self.tileArray`))) true true (struct :`G` 0.66 :`B` 1.0 :`A` 1.0) 5.0))

(fn `ConstructGrid`
  (for _index (range (`self.gridRows`))
    (for _index_2 (range (`self.gridCols`))
      (bind (_xpos _ypos) (`self.NewMacro` (`self.tileDim`) _index _index_2))
      (`self.Spawn Tile` _xpos _ypos _index _index_2)))
  (`KismetSystemLibrary.PrintString` "Grid Created"))

(fn `Spawn Tile`
  (params (xPos :type "Float (double-precision)") (yPos :type "Float (double-precision)") (rowIndex :type Integer) (colIndex :type Integer))
  (bind _returnvalue (`|SpawnActorFromClass` (`self.tileClass`) (`KismetMathLibrary.MakeTransform` (`KismetMathLibrary.MakeVector` xPos yPos)) "AlwaysSpawn" "MultiplyWithRoot" null null))
  (bind _asbp_tile (cast `/Game/Blueprints/Grid/BP_Tile` _returnvalue))
  (`/Game/Blueprints/Grid/BP_Tile.Init` _asbp_tile rowIndex colIndex (`self.tileDim`) (`self.shrinkFactor`))
  (`KismetArrayLibrary.Array_Add` (`self.tileArray`) _asbp_tile))

(fn `UpdateGrid`)

(fn `UserConstructionScript`)