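; Tower defence game mode that spawns the grid manager, creates the game UI and tracks score, health, wave and four resource types.
; Exclusive build, upgrade and destroy modes gate tower clicks.
; Selected towers come from seven per-type object pools, follow the hovered tile and activate when affordable, deducting resources and updating the grid.
; Tower upgrading is an empty stub, and destroying only calls DisableMessage, leaving refund logic unconnected.
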(event `self.ReceiveBeginPlay`
  (`self.SetUp`))

(fn `BuildTower`
  (params (incomingTower :type "/Game/Blueprints/Towers/BP_TowerBase Object Reference"))
  (bind _currenttile (`self.currentTile`))
  (bind _buildreqs (`/Game/Blueprints/Towers/BP_TowerBase.GetBuildResourceReqs` incomingTower))
  (bind _enoughresources (`self.CompareResourceReqs` _buildreqs))
  (if _enoughresources
    (`/Game/Blueprints/Towers/BP_TowerBase.ActivateTower` incomingTower _currenttile)
    (`/Game/Blueprints/Grid/BP_GridManager.UpdateTowerPlacements` (`self.gridManagerRef`) (`/Game/Blueprints/Grid/BP_Tile.gridPos` _currenttile))
    (set `self.selectedTower` null)
    (`self.SetResources` _buildreqs)))

(fn `CompareResourceReqs`
  (params (resourceReqs :type "Array of Integer"))
  (returns (enoughResources :type Boolean))
  (for (_array_element _array_index) resourceReqs
    (if (> _array_element (`|GetArrayItem` (`self.currentResources`) _array_index))
      (break)))
  (return (== _array_index (- (`KismetArrayLibrary.Array_Length` (`self.currentResources`)) 1))))

(fn `DestroyTower`
  (params (incomingTower :type "/Game/Blueprints/Towers/BP_TowerBase Object Reference"))
  (message `/Game/Blueprints/Helpers/BPI_PoolableObject.Disable` incomingTower))

(fn `ExitAllModes`
  (bind _currenttile (`self.currentTile`))
  (`self.SetModes` false)
  (`/Game/Blueprints/GUI/WBP_GameUI.UpdateToExitAllModes` (`self.GameUI`))
  (`/Engine/EditorBlueprintResources/StandardMacros.IsValid` _currenttile
    (:`Is Valid`
      (`/Game/Blueprints/Grid/BP_Tile.ChangeTileColour` _currenttile (`self.defaultTileColour`)))))

(fn `GetModes`
  (returns (BM :type Boolean) (UM :type Boolean) (DM :type Boolean))
  (return (`self.inBuildMode`) (`self.inUpgradeMode`) (`self.inDestroyMode`)))

(fn `GetTowerForUI`
  (params (towerType :type Integer))
  (returns (returnedObj :type "/Game/Blueprints/Towers/BP_TowerBase Object Reference"))
  (bind (_towerobj_g _towerobj_u _towerobj_a _towerobj_gu _towerobj_ga _towerobj_ua _towerobj_gua) (`self.TowerSelector` towerType)
    (:`Out Tower G`
      _)
    (:`Out Tower U`
      _)
    (:`Out Tower A`
      _)
    (:`Out Tower GU`
      _)
    (:`Out Tower GA`
      _)
    (:`Out Tower UA`
      _)
    (:`Out Tower GUA`
      _))
  (return (select `int` towerType :`0` _towerobj_g :`1` _towerobj_u :`2` _towerobj_a :`3` _towerobj_gu :`4` _towerobj_ga :`5` _towerobj_ua :`6` _towerobj_gua)))

(fn `GrabTower`
  (params (towerType :type Integer))
  (if (`self.inBuildMode`)
    (`self.ResetSelectedTower`)
    (bind (_towerobj_g _towerobj_u _towerobj_a _towerobj_gu _towerobj_ga _towerobj_ua _towerobj_gua) (`self.TowerSelector` towerType)
      (:`Out Tower G`
        (`self.SetSelectedTower` _towerobj_g))
      (:`Out Tower U`
        (`self.SetSelectedTower` _towerobj_u))
      (:`Out Tower A`
        (`self.SetSelectedTower` _towerobj_a))
      (:`Out Tower GU`
        (`self.SetSelectedTower` _towerobj_gu))
      (:`Out Tower GA`
        (`self.SetSelectedTower` _towerobj_ga))
      (:`Out Tower UA`
        (`self.SetSelectedTower` _towerobj_ua))
      (:`Out Tower GUA`
        (`self.SetSelectedTower` _towerobj_gua)))))

(fn `HoveringOverTile`
  (params (incomingTile :type "/Game/Blueprints/Grid/BP_Tile Object Reference"))
  (bind _currenttile (`self.currentTile`))
  (if (not (== incomingTile _currenttile))
    (`/Engine/EditorBlueprintResources/StandardMacros.IsValid` _currenttile
      (:`Is Valid`
        ;[1 1 1] Reverts previous tile's colour
        (`/Game/Blueprints/Grid/BP_Tile.ChangeTileColour` _currenttile (`self.defaultTileColour`)))
      (:`Is Not Valid`
        _))
    (`self.SetCurrentTile` incomingTile)
    (`self.MoveTowerToTile`)))

(fn `MoveTowerToTile`
  (bind _selectedtower (`self.selectedTower`))
  (`/Engine/EditorBlueprintResources/StandardMacros.IsValid` _selectedtower
    (:`Is Valid`
      (`self.K2_SetActorLocation` _selectedtower (`self.K2_GetActorLocation` (`self.currentTile`)) false true))))

(fn `OnTowerHoverStart`
  (params (inComingTower :type "/Game/Blueprints/Towers/BP_TowerBase Object Reference")))

(fn `OnTowerPressed`
  (params (incomingTower :type "/Game/Blueprints/Towers/BP_TowerBase Object Reference"))
  (bind _currenttile (`self.currentTile`))
  (if (`/Game/Blueprints/Towers/BP_TowerBase.isPlaced` incomingTower)
    (if (`self.inDestroyMode`)
      (`self.DestroyTower` incomingTower))
    (elif (`self.inBuildMode`)
      (if (and (`/Game/Blueprints/Grid/BP_Tile.canBuild` _currenttile) (not (`KismetSystemLibrary.IsValid` (`/Game/Blueprints/Grid/BP_Tile.occupant` _currenttile))))
        (`self.BuildTower` incomingTower)))))

(fn `RecoverInvestedResources`
  (params (incomingInvestedRes :type "Array of Integer") (recooveryExtent :type "Float (double-precision)"))
  (locals (recoveredResources :type "Array of Integer"))
  (for (_array_element _array_index) incomingInvestedRes
    (`KismetArrayLibrary.Array_Set` (`local.recoveredResources`) _array_index (`KismetMathLibrary.FTrunc` (* _array_element recooveryExtent))))
  (`self.SetResources` (`local.recoveredResources`) true))

(fn `ResetSelectedTower`
  (bind _selectedtower (`self.selectedTower`))
  (`/Engine/EditorBlueprintResources/StandardMacros.IsValid` _selectedtower
    (:`Is Valid`
      (message `/Game/Blueprints/Helpers/BPI_PoolableObject.Disable` _selectedtower)
      (set `self.selectedTower` null))))

(fn `SetBuildResAmt`
  (params (amountChange :type Integer))
  (bind _currentresources (`self.currentResources`))
  (bind _returnvalue (+ (`|GetArrayItem` _currentresources) amountChange))
  (`/Game/Blueprints/GUI/WBP_GameUI.UpdateBuildResourceAmt` (`self.GameUI`) _returnvalue)
  (`KismetArrayLibrary.Array_Set` _currentresources 0 _returnvalue))

(fn `SetCurrentTile`
  (params (inComing :type "/Game/Blueprints/Grid/BP_Tile Object Reference"))
  (bind _output_get (set `self.currentTile` inComing))
  (`KismetSystemLibrary.PrintString` (`KismetStringLibrary.Concat_StrStr` "Current Tile: " (`KismetSystemLibrary.GetDisplayName` _output_get)) true true (struct :`G` 0.66 :`B` 1.0 :`A` 1.0) 5.0))

(fn `SetHealth`
  (bind _healthcomp (`self.HealthComp`))
  (`/Game/Blueprints/GUI/WBP_GameUI.UpdateHealth` (`self.GameUI`) (/ (`/Game/Blueprints/Misc/AC_HealthComponent.currentHealth` _healthcomp) (`/Game/Blueprints/Misc/AC_HealthComponent.maxHealth` _healthcomp))))

(fn `SetScore`
  (params (scoreChange :type Integer))
  (bind _output_get (set `self.Score` (+ (`self.Score`) scoreChange)))
  (`/Game/Blueprints/GUI/WBP_GameUI.UpdateScore` (`self.GameUI`) _output_get))

(fn `SetToBuildMode`
  (if (`self.inBuildMode`)
    (`self.ExitAllModes`)
    (else
      (`self.SetModes` true)
      (`KismetSystemLibrary.PrintString` "InBuildMode")
      (`/Game/Blueprints/GUI/WBP_GameUI.UpdateToBuildMode` (`self.GameUI`))))
  (`self.ResetSelectedTower`))

(fn `SetToDestroyMode`
  (if (`self.inDestroyMode`)
    (`self.ExitAllModes`)
    (else
      (`self.SetModes` false false true)
      (`KismetSystemLibrary.PrintString` "In Destroy Mode")
      (`/Game/Blueprints/GUI/WBP_GameUI.UpdateToDestroyMode` (`self.GameUI`))
      (`self.ResetSelectedTower`))))

(fn `SetToUpgradeMode`
  (if (`self.inUpgradeMode`)
    (`self.ExitAllModes`)
    (else
      (`self.SetModes` false true)
      (`KismetSystemLibrary.PrintString` "InUpgradeMode")
      (`/Game/Blueprints/GUI/WBP_GameUI.UpdateToUpgradeMode` (`self.GameUI`))
      (`self.ResetSelectedTower`))))

(fn `SetUp`
  (bind _returnvalue (`|SpawnActorFromClass` "/Game/Blueprints/Grid/BP_GridManager.BP_GridManager_C" (`KismetMathLibrary.MakeTransform` (0.0 0.0 500.0)) "Undefined" "MultiplyWithRoot" null null))
  (set `self.gridManagerRef` _returnvalue)
  ;[1 1 1] Creates the GUI
  (bind _returnvalue_2 (`|CreateWidget` "/Game/Blueprints/GUI/WBP_GameUI.WBP_GameUI_C"))
  (bind _output_get (set `self.GameUI` _returnvalue_2))
  (`UserWidget.AddToViewport` _output_get 0)
  (`KismetSystemLibrary.PrintString` "Added GameUI")
  ;[1 1 1] Sets starting score to 0
  (set `self.Score` 0)
  (`self.SetScore` 0)
  (`/Game/Blueprints/Misc/AC_HealthComponent.Init` (`self.HealthComp`)))

(fn `SetUpgradeRes1Amt`
  (params (changeAmount :type Integer))
  (bind _currentresources (`self.currentResources`))
  (bind _returnvalue (+ (`|GetArrayItem` _currentresources 1) changeAmount))
  (`/Game/Blueprints/GUI/WBP_GameUI.UpdateUpgradeResourceGAmt` (`self.GameUI`) _returnvalue)
  (`KismetArrayLibrary.Array_Set` _currentresources 1 _returnvalue))

(fn `SetUpgradeRes2Amt`
  (params (changeAmount :type Integer))
  (bind _currentresources (`self.currentResources`))
  (bind _returnvalue (+ (`|GetArrayItem` _currentresources 2) changeAmount))
  (`/Game/Blueprints/GUI/WBP_GameUI.UpdateUpgradeResourceUAmt` (`self.GameUI`) _returnvalue)
  (`KismetArrayLibrary.Array_Set` _currentresources 2 _returnvalue))

(fn `SetUpgradeRes3Amt`
  (params (changeAmount :type Integer))
  (bind _currentresources (`self.currentResources`))
  (bind _returnvalue (+ (`|GetArrayItem` _currentresources 3) changeAmount))
  (`/Game/Blueprints/GUI/WBP_GameUI.UpdateUpgradeResourceAAmt` (`self.GameUI`) _returnvalue)
  (`KismetArrayLibrary.Array_Set` _currentresources 3 _returnvalue))

(fn `SetWave`
  (`/Game/Blueprints/GUI/WBP_GameUI.UpdateWave` (`self.GameUI`) (`self.currentWave`)))

(fn `UpgradeTower`)

(fn `UserConstructionScript`)