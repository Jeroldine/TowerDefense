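; Player camera pawn that handles panning, zooming and switching between build, upgrade and destroy modes.
; Zoom input moves the pawn along the camera's forward vector, while panning works only with the pan key held.
; Panning follows the actor's right vector, clamps Y position and zeroes velocity at limits, with the upper bound settable through Init.
; Mode inputs toggle mutually exclusive flags and print the entered mode.
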(event `self.ReceiveBeginPlay`
  ;[1 1 1] Initialization
  (set `PlayerController.bShowMouseCursor` true (`GameplayStatics.GetPlayerController` 0)))

(event `InputAction|EnterPanMode`
  (params (Key :type "Key Structure"))
  ;[1 1 1] Allow Panning
  (:`Pressed`
    (set `self.canPan` true))
  (:`Released`
    (set `self.canPan` false)))

(event `InputAction|ZoomIn`
  (params (Key :type "Key Structure"))
  ;[1 1 1] Zoom in and out
  (:`Pressed`
    (`self.AddMovementInput` (`SceneComponent.GetForwardVector` (`self.Camera`)) (`self.zoomSpeed`))))

(event `InputAction|ZoomOut`
  (params (Key :type "Key Structure"))
  ;[1 1 1] Zoom in and out
  (:`Pressed`
    (`self.AddMovementInput` (`SceneComponent.GetForwardVector` (`self.Camera`)) (* (`self.zoomSpeed`) -1.0))))

(event `InputAxis|PanRight`
  (params (AxisValue :type "Float (single-precision)"))
  ;[1 1 1] Panning Movement
  (`self.PanCamera` AxisValue))

(event `InputAction|EnterBuildMode`
  (params (Key :type "Key Structure"))
  ;[1 1 1] Switch between modes
  (:`Pressed`
    (`self.OnEnterBuildMode`)))

(event `InputAction|EnterUpgradeMode`
  (params (Key :type "Key Structure"))
  ;[1 1 1] Switch between modes
  (:`Pressed`
    (`self.OnEnterUpgradeMode`)))

(event `InputAction|EnterDestroyMode`
  (params (Key :type "Key Structure"))
  ;[1 1 1] Switch between modes
  (:`Pressed`
    (`self.OnEnterDestroyMode`)))

(fn `ExitAllModes`
  (set `self.inBuildMode` false)
  (set `self.inUpgradeMode` false)
  (set `self.inDestroyMode` false))

(fn `Init`
  (params (yPosMax :type "Float (double-precision)"))
  (set `self.yPosMax` yPosMax))

(fn `OnEnterBuildMode`
  (if (`self.inBuildMode`)
    (`self.ExitAllModes`)
    (else
      (set `self.inBuildMode` true)
      (set `self.inUpgradeMode` false)
      (set `self.inDestroyMode` false)
      (`KismetSystemLibrary.PrintString` "In Build Mode"))))

(fn `OnEnterDestroyMode`
  (if (`self.inDestroyMode`)
    (`self.ExitAllModes`)
    (else
      (set `self.inBuildMode` false)
      (set `self.inUpgradeMode` false)
      (set `self.inDestroyMode` true)
      (`KismetSystemLibrary.PrintString` "In Destroy Mode"))))

(fn `OnEnterUpgradeMode`
  (if (`self.inUpgradeMode`)
    (`self.ExitAllModes`)
    (else
      (set `self.inBuildMode` false)
      (set `self.inUpgradeMode` true)
      (set `self.inDestroyMode` false)
      (`KismetSystemLibrary.PrintString` "In Upgrade Mode"))))

(fn `PanCamera`
  (params (dir :type "Float (double-precision)"))
  (bind (_returnvalue_x _returnvalue_y _returnvalue_z) (`KismetMathLibrary.BreakVector` (`self.K2_GetActorLocation`)))
  (bind (_returnvalue_x_2 _returnvalue_y_2 _returnvalue_z_2) (`KismetMathLibrary.BreakVector` (`self.K2_GetActorLocation`)))
  (bind _yposmin (`self.yPosMin`))
  (bind _yposmax (`self.yPosMax`))
  (if (`self.canPan`)
    (`self.AddMovementInput` (`self.GetActorRightVector`) (* (`self.panSpeed`) dir -1.0))
    (if (< _returnvalue_y_2 _yposmin)
      (`self.K2_SetActorLocation` (`KismetMathLibrary.MakeVector` _returnvalue_x_2 _yposmin _returnvalue_z_2))
      (set `MovementComponent.Velocity` (0.0 0.0 0.0) (`self.FloatingPawnMovement`))
      (elif (> _returnvalue_y _yposmax)
        (`self.K2_SetActorLocation` (`KismetMathLibrary.MakeVector` _returnvalue_x _yposmax _returnvalue_z))
        (set `MovementComponent.Velocity` (0.0 0.0 0.0) (`self.FloatingPawnMovement`))))))

(fn `UserConstructionScript`)