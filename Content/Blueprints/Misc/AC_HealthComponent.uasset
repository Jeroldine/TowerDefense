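; AC_HealthComponent is an actor component that tracks a health value for its owner.
; Init sets CurrentHealth to MaxHealth, while Damage and Heal subtract or add an amount, clamped between zero and MaxHealth.
; BeginPlay and Tick are unused, and the component itself never calls Init or reacts when health reaches zero.
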(fn `Damage`
  (params (dmgAmount :type "Float (double-precision)"))
  (set `self.currentHealth` (`KismetMathLibrary.FClamp` (- (`self.currentHealth`) dmgAmount) 0.0 (`self.maxHealth`))))

(fn `Heal`
  (params (healAmount :type "Float (double-precision)"))
  (set `self.currentHealth` (`KismetMathLibrary.FClamp` (+ (`self.currentHealth`) healAmount) 0.0 (`self.maxHealth`))))

(fn `Init`
  (set `self.currentHealth` (`self.maxHealth`)))