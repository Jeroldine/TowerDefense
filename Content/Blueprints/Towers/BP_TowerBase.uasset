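; Base tower Blueprint that provides mouse interaction and object pooling hooks, presumably for child towers to override.
; Click, hover and pool events forward to matching functions, all empty except OnDisable.
; OnDisable parks the actor below the world at a fixed negative Z, limits PawnSensing to players only, and turns off visibility, collision and tick rather than destroying it.
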(event `/Game/Blueprints/Helpers/BPI_InteractableObject.MouseClicked`
  ;[1 1 1] Mouse Interactions
  (`self.OnMouseClicked`))

(event `/Game/Blueprints/Helpers/BPI_PoolableObject.Initialize`
  ;[1 1 1] Poolable Object Functionality
  (`self.OnInitialize`))

(event `/Game/Blueprints/Helpers/BPI_InteractableObject.MouseHoverStart`
  ;[1 1 1] Mouse Interactions
  (`self.OnMouseHoverStart`))

(event `/Game/Blueprints/Helpers/BPI_PoolableObject.Disable`
  ;[1 1 1] Poolable Object Functionality
  (`self.On Disable`))

(event `/Game/Blueprints/Helpers/BPI_InteractableObject.MouseHoverEnd`
  ;[1 1 1] Mouse Interactions
  (`self.OnMouseHoverEnd`))

(fn `On Disable`
  (bind (_returnvalue_x _returnvalue_y) (`KismetMathLibrary.BreakVector` (`self.K2_GetActorLocation`)))
  (`self.K2_SetActorLocation` (`KismetMathLibrary.MakeVector` _returnvalue_x _returnvalue_y -500.0) false true)
  (set `PawnSensingComponent.bOnlySensePlayers` true (`self.PawnSensing`))
  (`self.SetActorHiddenInGame` true)
  (`self.SetActorEnableCollision` false)
  (`self.SetActorTickEnabled` false))

(fn `OnInitialize`)

(fn `OnMouseClicked`)

(fn `OnMouseHoverEnd`)

(fn `OnMouseHoverStart`)

(fn `UserConstructionScript`)