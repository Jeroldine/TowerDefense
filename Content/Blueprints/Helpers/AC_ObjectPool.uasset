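; Actor component that serves as an object pool, pre-spawning a starting number of actors of a configurable class.
; On BeginPlay, Init repeatedly calls CreateSingleObject, which spawns an actor at the world origin.
; Each spawn implementing BPI_PoolableObject is disabled through an interface message and added to the pool array.
; SpawnObject is an empty stub, so nothing here retrieves pooled objects yet.
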(event `self.ReceiveBeginPlay`
  (`self.Init`))

(fn `CreateSingleObject`
  (bind _returnvalue (`|SpawnActorFromClass` (`self.objType`) (`KismetMathLibrary.MakeTransform` (0.0 0.0 0.0)) "AdjustIfPossibleButAlwaysSpawn" "MultiplyWithRoot" null null))
  (bind _asbpi_poolable_object (cast `/Game/Blueprints/Helpers/BPI_PoolableObject` _returnvalue))
  (message `/Game/Blueprints/Helpers/BPI_PoolableObject.Disable` _returnvalue)
  (`KismetArrayLibrary.Array_Add` (`self.objPool`) _asbpi_poolable_object))

(fn `Init`
  (for _ (range (`self.startingNumber`))
    (`self.CreateSingleObject`)))

(fn `SpawnObject`)