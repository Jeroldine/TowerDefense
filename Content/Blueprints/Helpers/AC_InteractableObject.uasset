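; Actor component that makes its owning actor respond to mouse clicks and hovering.
; On BeginPlay it binds to the owner's OnClicked, OnBeginCursorOver and OnEndCursorOver events.
; Each handler prints a debug string, then forwards a matching message to the owner if it implements BPI_InteractableObject.
; MouseClicked, MouseHoverStart and MouseHoverEnd functions in the component are empty.
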(event `self.ReceiveBeginPlay`
  (bind _returnvalue (`self.GetOwner`))
  (add `Actor.OnClicked` _returnvalue (delegate `Clicked`))
  (add `Actor.OnBeginCursorOver` _returnvalue (delegate `HoverStart`))
  (add `Actor.OnEndCursorOver` _returnvalue (delegate `HoverEnd`)))

(event `Clicked`
  (params (TouchedActor :type "Actor Object Reference") (ButtonPressed :type "Key Structure" :default "None"))
  (`self.ClickBind`))

(event `HoverStart`
  (params (TouchedActor :type "Actor Object Reference"))
  (`self.Hover Start Bind`))

(event `HoverEnd`
  (params (TouchedActor :type "Actor Object Reference"))
  (`self.Hover End Bind`))

(fn `ClickBind`
  (bind _returnvalue (`self.GetOwner`))
  (`KismetSystemLibrary.PrintString` "InteractableObject clicked")
  (cast `/Game/Blueprints/Helpers/BPI_InteractableObject` _returnvalue)
  (message `/Game/Blueprints/Helpers/BPI_InteractableObject.MouseClicked` _returnvalue))

(fn `Hover End Bind`
  (bind _returnvalue (`self.GetOwner`))
  (`KismetSystemLibrary.PrintString` "InteractableObject NOT hovered over")
  (cast `/Game/Blueprints/Helpers/BPI_InteractableObject` _returnvalue)
  (message `/Game/Blueprints/Helpers/BPI_InteractableObject.MouseHoverEnd` _returnvalue))

(fn `Hover Start Bind`
  (bind _returnvalue (`self.GetOwner`))
  (`KismetSystemLibrary.PrintString` "InteractableObject hovered over")
  (cast `/Game/Blueprints/Helpers/BPI_InteractableObject` _returnvalue)
  (message `/Game/Blueprints/Helpers/BPI_InteractableObject.MouseHoverStart` _returnvalue))

(fn `MouseClicked`)

(fn `MouseHoverEnd`)

(fn `MouseHoverStart`)