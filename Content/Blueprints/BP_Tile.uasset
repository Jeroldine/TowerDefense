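; BP_Tile is a single grid tile actor that stores its row and column and sizes its cube mesh to a requested tile dimension.
; Init saves the coordinates, then uniformly scales the Cube by the target size divided by the mesh's native width, multiplied by a shrink factor.
; GetCubeDim derives that native width from the static mesh bounds, so the sizing adapts to whichever mesh is assigned.
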(event `self.ReceiveBeginPlay`)

(fn `GetCubeDim`
  (returns (CubeSideLength :type "Float (double-precision)"))
  (return (* (.x (`.BoxExtent` (`KismetMathLibrary.BreakBoxSphereBounds` (`StaticMesh.GetBounds` (`StaticMeshComponent.StaticMesh` (`self.Cube`)))))) 2.0)))

(fn `Init`
  (params (row :type Integer) (col :type Integer) (newTileDim :type "Float (double-precision)") (shrinkFactor :type "Float (double-precision)"))
  (set `self.row` row)
  (set `self.col` col)
  (`SceneComponent.SetRelativeScale3D` (`self.Cube`) (`KismetMathLibrary.Conv_DoubleToVector` (* (`KismetMathLibrary.SafeDivide` newTileDim (`self.GetCubeDim`)) shrinkFactor))))

(fn `UserConstructionScript`)